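; BP_AI_Player is the AI-driven monster that hunts BP_AI_NonPlayer characters, running BT_AI_Player.
; A vision cone maintains the tracked list; Tick writes the nearest living target to the blackboard as Prey when not attacking.
; OrderToKill temporarily locks Prey to the top-down controller's selected target.
; Ability events temporarily boost vision or speed, while ShadowWizardry kills every listed AI after a delay, with radial force and sounds.
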(event OnComponentBeginOverlap(MainVisionCone)
  (params (OverlappedComponent :type Primitive%20Component%20Object%20Reference) (OtherActor :type Actor%20Object%20Reference) (OtherComp :type Primitive%20Component%20Object%20Reference) (OtherBodyIndex :type Integer) (bFromSweep :type Boolean) (SweepResult :type Hit%20Result%20Structure%20%28by%20ref%29))
  (if (== OtherComp (Actor|GetComponentbyClass OtherActor "/Script/Engine.CapsuleComponent"))
    (bind _asbp_ai_non_player (Utilities|Casting|CastToBP_AI_NonPlayer OtherActor))
    (if (Variables|/Game/Blueprints/AI_Folder/BP_AI_Parent.BP_AI_Parent_C|GetIsAlive _asbp_ai_non_player)
      (Utilities|Array|Add (Variables|Default|GetListAITracking) _asbp_ai_non_player))))

(event OnComponentEndOverlap(MainVisionCone)
  (params (OverlappedComponent :type Primitive%20Component%20Object%20Reference) (OtherActor :type Actor%20Object%20Reference) (OtherComp :type Primitive%20Component%20Object%20Reference) (OtherBodyIndex :type Integer))
  (if (== OtherComp (Actor|GetComponentbyClass OtherActor "/Script/Engine.CapsuleComponent"))
    (bind _asbp_ai_non_player (Utilities|Casting|CastToBP_AI_NonPlayer OtherActor))
    (Utilities|Array|RemoveItem (Variables|Default|GetListAITracking) _asbp_ai_non_player)))

(event Custom|EnhanceSpeed
  (bind _charactermovement (Variables|Character|GetCharacterMovement))
  (Variables|/Script/Engine.CharacterMovementComponent|SetMaxWalkSpeed _charactermovement 1.2e+03)
  (Utilities|FlowControl|Delay 1e+01)
  (Variables|/Script/Engine.CharacterMovementComponent|SetMaxWalkSpeed _charactermovement 6e+02))

(event Custom|EnhanceSense
  (bind _mainvisioncone (Variables|Default|GetMainVisionCone))
  (bind _mainvisioncone_2 (Variables|Default|GetMainVisionCone))
  (bind _returnvalue (Transformation|GetWorldTransform _mainvisioncone_2))
  (bind _returnvalue_2 (Transformation|GetWorldTransform _mainvisioncone))
  (bind (_location _rotation _scale) (Math|Transform|BreakTransform _returnvalue_2))
  (bind (_location_2 _rotation_2 _scale_2) (Math|Transform|BreakTransform _returnvalue))
  (Transformation|SetWorldTransform _mainvisioncone (Math|Transform|MakeTransform _location _rotation (* _scale 2.0)) false false)
  (Utilities|FlowControl|Delay 1e+01)
  (Transformation|SetWorldTransform _mainvisioncone_2 (Math|Transform|MakeTransform _location_2 _rotation_2 (* _scale_2 0.5)) false false))

(event Custom|ShadowWizardry
  (bind _asbp_game_instance (Utilities|Casting|CastToBP_GameInstance (Game|GetGameInstance)))
  (Audio|PlaySound2D "/Game/Audio/FX/SW_ShadowBombTick.SW_ShadowBombTick" 1.0 1.0 0.0 0 0)
  (Utilities|FlowControl|Delay 2.1)
  (for _array_element (Variables|/Game/Blueprints/Misc/BP_GameInstance.BP_GameInstance_C|GetListOfAllAI _asbp_game_instance)
    (if (Variables|/Game/Blueprints/AI_Folder/BP_AI_Parent.BP_AI_Parent_C|GetIsAlive _array_element)
      (Variables|/Game/Blueprints/AI_Folder/BP_AI_Parent.BP_AI_Parent_C|SetHealth _array_element -100)))
  (Components|Activation|Activate (Variables|Default|GetRadialForce) false)
  (Audio|PlaySound2D "/Game/Audio/FX/SW_ShadowScream.SW_ShadowScream" 1.0 1.0 0.0 0 0)
  (Development|PrintString "I love casting spell"))

(event Custom|OrderToKill
  (bind _astop_down_controller (Utilities|Casting|CastToTopDownController (Game|GetPlayerController 0)))
  (if (Variables|/Game/Blueprints/AI_Folder/BP_AI_Parent.BP_AI_Parent_C|GetIsAlive (Variables|/Game/Blueprints/TopDownController.TopDownController_C|GetTargetSelected _astop_down_controller))
    (Variables|Default|SetCanChangePrey false)
    (Utilities|FlowControl|Delay 0.2)
    (Variables|Default|SetPrey (Variables|/Game/Blueprints/TopDownController.TopDownController_C|GetTargetSelected _astop_down_controller))
    (Utilities|FlowControl|Delay 1e+01)
    (Variables|Default|SetCanChangePrey true)))

(event EventTick
  (params (DeltaSeconds :type Float%20%28single-precision%29))
  (bind _self self)
  (bind _listaitracking (Variables|Default|GetListAITracking))
  (|CallParentFunction 0.0)
  (if true
    (if (not (Variables|Default|GetCurrentlyAttacking))
      (if (Variables|Default|GetCanChangePrey)
        (if (Utilities|Array|IsValidIndex _listaitracking) :!label _label
          (Variables|Default|SetPrey (Utilities|Array|Get(acopy) _listaitracking))
          (for _array_element _listaitracking
            (if (Variables|/Game/Blueprints/AI_Folder/BP_AI_Parent.BP_AI_Parent_C|GetIsAlive _array_element)
              (if (< (Transformation|GetDistanceTo _array_element _self) (Transformation|GetDistanceTo (Variables|Default|GetPrey) _self))
                (Variables|Default|SetPrey _array_element))
              (else
                (Utilities|Array|RemoveItem _listaitracking _array_element))))
          (AI|Components|Blackboard|SetValueasObject (stale EventBeginPlay _blackboardcomponent) (Utilities|Name|MakeLiteralName "Prey") (Variables|Default|GetPrey) :!label _label_2)
          (elif (Utilities|IsValid (Variables|Default|GetPrey))
            (Variables|Default|SetPrey 0)
            (AI|Components|Blackboard|SetValueasObject (stale EventBeginPlay _blackboardcomponent) (Utilities|Name|MakeLiteralName "Prey") 0)))
        (elif (Variables|/Game/Blueprints/AI_Folder/BP_AI_Parent.BP_AI_Parent_C|GetIsAlive (Variables|Default|GetPrey))
          (goto _label_2)
          (else
            (Variables|Default|SetCanChangePrey true)
            (goto _label)))))))

(event EventBeginPlay
  (|CallParentFunction)
  (bind _asaicontroller (Utilities|Casting|CastToAIController (Pawn|GetController)))
  (AI|RunBehaviorTree _asaicontroller "/Game/Blueprints/AI_Folder/AI_Player/BT_AI_Player.BT_AI_Player")
  (bind _blackboardcomponent (Class|AIController|UseBlackboard _asaicontroller "/Game/Blueprints/AI_Folder/AI_Player/BB_AI_Player.BB_AI_Player"))
  (Variables|Default|SetTags (Utilities|Array|MakeArray "Monster")))

(fn ConstructionScript
  (|CallParentFunction))