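; Non-civilian NPC AI that turns hostile toward the Predator, running BT_AI_NonCivil with the BB_NonPlayer blackboard seeded at BeginPlay.
; While idle, its vision cone triggers attack mode on seeing the Predator, an alerted NPC, or a dead idle one, updating the blackboard and movement speed.
; While alert, Tick rotates the capsule toward the Predator and resets IsIdle once it dies, without updating the blackboard.
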(event OnComponentBeginOverlap(MainVisionCone)
  (params (OverlappedComponent :type Primitive%20Component%20Object%20Reference) (OtherActor :type Actor%20Object%20Reference) (OtherComp :type Primitive%20Component%20Object%20Reference) (OtherBodyIndex :type Integer) (bFromSweep :type Boolean) (SweepResult :type Hit%20Result%20Structure%20%28by%20ref%29))
  (bind _charactermovement (Variables|Character|GetCharacterMovement))
  (if (Variables|Default|GetIsIdle)
    (if (== OtherComp (Actor|GetComponentbyClass OtherActor "/Script/Engine.CapsuleComponent"))
      (if (== OtherActor (Variables|Default|GetPredator))
        (Variables|Default|SetIsIdle false :!label _label)
        (AI|Components|Blackboard|SetValueasBool (stale EventBeginPlay _blackboardcomponent) (Utilities|Name|MakeLiteralName "IsIdle") (Variables|Default|GetIsIdle))
        (Variables|/Script/Engine.CharacterMovementComponent|SetMaxWalkSpeed _charactermovement 6e+02)
        (Variables|/Script/Engine.CharacterMovementComponent|SetMaxAcceleration _charactermovement 2048.0)
        (Development|PrintString "Attacking")
        (else
          (bind _asbp_ai_non_player (Utilities|Casting|CastToBP_AI_NonPlayer OtherActor))
          (if (Variables|/Game/Blueprints/AI_Folder/BP_AI_Parent.BP_AI_Parent_C|GetIsIdle _asbp_ai_non_player)
            (if (not (Variables|/Game/Blueprints/AI_Folder/BP_AI_Parent.BP_AI_Parent_C|GetIsAlive _asbp_ai_non_player))
              (goto _label))
            (else
              (goto _label))))))))

(event EventBeginPlay
  (|CallParentFunction)
  (bind _asaicontroller (Utilities|Casting|CastToAIController (Pawn|GetController)))
  (AI|RunBehaviorTree _asaicontroller "/Game/Blueprints/AI_Folder/AI_NonPlayer/AI_NonCivil_Folder/BT_AI_NonCivil.BT_AI_NonCivil")
  (bind _blackboardcomponent (Class|AIController|UseBlackboard _asaicontroller "/Game/Blueprints/AI_Folder/AI_NonPlayer/BB_NonPlayer.BB_NonPlayer"))
  (AI|Components|Blackboard|SetValueasBool _blackboardcomponent (Utilities|Name|MakeLiteralName "IsAlive") (Variables|Default|GetIsAlive))
  (AI|Components|Blackboard|SetValueasBool _blackboardcomponent (Utilities|Name|MakeLiteralName "IsIdle") (Variables|Default|GetIsIdle))
  (Class|BlackboardComponent|SetValueasInt _blackboardcomponent (Utilities|Name|MakeLiteralName "Type") (Variables|Default|GetType))
  (AI|Components|Blackboard|SetValueasObject _blackboardcomponent (Utilities|Name|MakeLiteralName "SelfActor") self))

(event EventTick
  (params (DeltaSeconds :type Float%20%28single-precision%29))
  (bind _capsulecomponent (Variables|Default|GetCapsuleComponent))
  (|CallParentFunction 0.0)
  (if (not (Variables|Default|GetIsIdle))
    (Transformation|SetWorldRotation _capsulecomponent (Math|Rotator|FindLookatRotation (Transformation|GetWorldLocation _capsulecomponent) (Transformation|GetWorldLocation (Variables|/Script/Engine.Character|GetCapsuleComponent (Variables|Default|GetPredator)))) false false)
    (if (not (Variables|/Game/Blueprints/AI_Folder/BP_AI_Parent.BP_AI_Parent_C|GetIsAlive (Variables|Default|GetPredator)))
      (Variables|Default|SetIsIdle true))))

(fn ConstructionScript
  (|CallParentFunction))