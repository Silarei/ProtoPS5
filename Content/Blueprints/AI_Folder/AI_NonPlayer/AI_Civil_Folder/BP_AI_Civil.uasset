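; BP_AI_Civil is a civilian NPC character run by the BT_AI_Civil behavior tree.
; On BeginPlay it seeds the BB_NonPlayer blackboard with alive, idle, type and self values.
; A player capsule entering its vision cone is stored as Predator, ending idle and setting movement speed and acceleration.
; A once-only Tick check marks it dead at zero health and disables capsule collision, without updating the blackboard here.
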(event OnComponentBeginOverlap(MainVisionCone)
  (params (OverlappedComponent :type Primitive%20Component%20Object%20Reference) (OtherActor :type Actor%20Object%20Reference) (OtherComp :type Primitive%20Component%20Object%20Reference) (OtherBodyIndex :type Integer) (bFromSweep :type Boolean) (SweepResult :type Hit%20Result%20Structure%20%28by%20ref%29))
  (bind _charactermovement (Variables|Character|GetCharacterMovement))
  (if (== OtherComp (Actor|GetComponentbyClass OtherActor "/Script/Engine.CapsuleComponent"))
    (bind _asbp_ai_player (Utilities|Casting|CastToBP_AI_Player OtherActor))
    (bind _output_get (Variables|Default|SetPredator _asbp_ai_player))
    (Development|PrintString (Utilities|GetDisplayName _output_get))
    (Variables|Default|SetIsIdle false)
    (Variables|/Script/Engine.CharacterMovementComponent|SetMaxWalkSpeed _charactermovement 6e+02)
    (Variables|/Script/Engine.CharacterMovementComponent|SetMaxAcceleration _charactermovement 2048.0)))

(event EventBeginPlay
  (bind _asaicontroller (Utilities|Casting|CastToAIController (Pawn|GetController)))
  (AI|RunBehaviorTree _asaicontroller "/Game/Blueprints/AI_Folder/AI_NonPlayer/AI_Civil_Folder/BT_AI_Civil.BT_AI_Civil")
  (bind _blackboardcomponent (Class|AIController|UseBlackboard _asaicontroller "/Game/Blueprints/AI_Folder/AI_NonPlayer/BB_NonPlayer.BB_NonPlayer"))
  (AI|Components|Blackboard|SetValueasBool _blackboardcomponent (Utilities|Name|MakeLiteralName "IsAlive") (Variables|Default|GetIsAlive))
  (AI|Components|Blackboard|SetValueasBool _blackboardcomponent (Utilities|Name|MakeLiteralName "IsIdle") (Variables|Default|GetIsIdle))
  (Class|BlackboardComponent|SetValueasInt _blackboardcomponent (Utilities|Name|MakeLiteralName "Type") (Variables|Default|GetType))
  (AI|Components|Blackboard|SetValueasObject _blackboardcomponent (Utilities|Name|MakeLiteralName "SelfActor") self))

(event EventTick
  (params (DeltaSeconds :type Float%20%28single-precision%29))
  (if (not (> (Variables|Default|GetHealth) 0))
    (Utilities|FlowControl|DoOnce false
      (:Completed
        (Variables|Default|SetIsAlive false)
        (Rendering|ToggleVisibility (Variables|Default|GetCapsuleComponent) true)
        (Collision|SetCollisionEnabled (Variables|Default|GetCapsuleComponent) "NoCollision")))))

(fn ConstructionScript
  (|CallParentFunction))